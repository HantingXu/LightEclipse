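; Elevator that travels up or down a set distance when the player enters its trigger box, first animating an optional floor switch.
; An OnElevatorStatusChanged dispatcher drives the switch reset and a shared travel timeline, with a multiplier setting direction.
; BeginPlay tiles "Chain"-tagged meshes into segments attached to the platform, hiding those that rise above the top of travel.
; The construction script toggles an optional spotlight.
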(event OnComponentBeginOverlap(Box)
  (params (OverlappedComponent :type Primitive%20Component%20Object%20Reference) (OtherActor :type Actor%20Object%20Reference) (OtherComp :type Primitive%20Component%20Object%20Reference) (OtherBodyIndex :type Integer) (bFromSweep :type Boolean) (SweepResult :type Hit%20Result%20Structure%20%28by%20ref%29))
  (if (and (== OtherActor (Game|GetPlayerCharacter 0)) (or (Utilities|Enum|Equal(Enum) (Variables|Initialization|GetElevator%20Status) "NewEnumerator0") (Utilities|Enum|Equal(Enum) (Variables|Initialization|GetElevator%20Status) "NewEnumerator3")))
    (if (Utilities|IsValid (Variables|/Script/Engine.StaticMeshComponent|GetStaticMesh (Variables|Default|GetElevator%20Switch)))
      (bind _switch_movement_z_axis (Timeline|ElevatorSwitch PlayFromStart)
        (:Update
          (Transformation|SetRelativeLocation (Variables|Default|GetElevator%20Switch) (Math|Vector|MakeVector 0.0 0.0 _switch_movement_z_axis) false true))
        (:Finished
          (if (Utilities|Enum|Equal(Enum) (Variables|Initialization|GetElevator%20Status) "NewEnumerator0") :!label _label
            (bind _output_get (Variables|Initialization|SetElevator%20Status "NewEnumerator2"))
            (Default|CallOnElevatorStatusChanged _output_get)
            (else
              (bind _output_get_2 (Variables|Initialization|SetElevator%20Status "NewEnumerator1"))
              (Default|CallOnElevatorStatusChanged _output_get_2)))))
      (else
        (goto _label)))))

(event Custom|Elevator%20Go%20Up
  (bind _distance_to_travel (Variables|Initialization|GetDistance%20To%20Travel))
  (Components|Timeline|SetPlayRate (Variables|Default|GetElevator%20Travel) (Variables|Initialization|GetTravel%20Speed))
  (Variables|Default|SetMultiplier 1.0)
  (bind _elevator_z_axis (Timeline|Elevator%20Travel PlayFromStart)
    (:Update
      (Transformation|SetWorldLocation (Variables|Default|GetSM_Elevator_1) (+ (Variables|Default|GetElevator%20Start%20Location) (Math|Vector|MakeVector 0.0 0.0 (* _elevator_z_axis _distance_to_travel (Variables|Default|GetMultiplier)))) false true)
      (for _array_element (Variables|Default|GetAll%20Static%20Meshes)
        (if (Utilities|Enum|Equal(Enum) (Variables|Initialization|GetElevator%20Status) "NewEnumerator2")
          (if (> (.Z (Math|Vector|BreakVector (Transformation|GetWorldLocation _array_element))) (.z (+ (Variables|Default|GetElevator%20Start%20Location) (Math|Vector|MakeVector 0.0 0.0 _distance_to_travel))))
            (Rendering|SetVisibility _array_element false false)
            (else
              (Rendering|SetVisibility _array_element true false :!label _label)))
          (else
            (goto _label)))))
    (:Finished
      (if (Utilities|Enum|Equal(Enum) (Variables|Initialization|GetElevator%20Status) "NewEnumerator2")
        (bind _output_get (Variables|Initialization|SetElevator%20Status "NewEnumerator3"))
        (Default|CallOnElevatorStatusChanged _output_get)
        (else
          (bind _output_get_2 (Variables|Initialization|SetElevator%20Status "NewEnumerator0"))
          (Default|CallOnElevatorStatusChanged _output_get_2)))
      (Variables|Default|SetElevator%20Start%20Location (Transformation|GetWorldLocation (Variables|Default|GetSM_Elevator_1))))))

(event Custom|On%20Elevator%20Status%20Changed_Event
  (params (New%20elevator%20Status :type E_ElevatorStatus%20Enum :default "NewEnumerator0"))
  (switch Utilities|FlowControl|Switch|SwitchonE_ElevatorStatus New%20elevator%20Status
    (:NewEnumerator0
      (bind _switch_movement_z_axis (Timeline|Timeline_0 PlayFromStart)
        (:Update
          (Transformation|SetRelativeLocation (Variables|Default|GetElevator%20Switch) (Math|Vector|MakeVector 0.0 0.0 _switch_movement_z_axis) false true))))
    (:NewEnumerator1
      (CallFunction|ElevatorGoDown))
    (:NewEnumerator2
      (CallFunction|ElevatorGoUp))
    (:NewEnumerator3
      (Timeline|Timeline_0 PlayFromStart))))

(event Custom|Elevator%20Go%20Down
  (bind _distance_to_travel (Variables|Initialization|GetDistance%20To%20Travel))
  (Components|Timeline|SetPlayRate (Variables|Default|GetElevator%20Travel) (Variables|Initialization|GetTravel%20Speed))
  (Variables|Default|SetMultiplier -1.0)
  (bind _elevator_z_axis (Timeline|Elevator%20Travel PlayFromStart)
    (:Update
      (Transformation|SetWorldLocation (Variables|Default|GetSM_Elevator_1) (+ (Variables|Default|GetElevator%20Start%20Location) (Math|Vector|MakeVector 0.0 0.0 (* _elevator_z_axis _distance_to_travel (Variables|Default|GetMultiplier)))) false true)
      (for _array_element (Variables|Default|GetAll%20Static%20Meshes)
        (if (Utilities|Enum|Equal(Enum) (Variables|Initialization|GetElevator%20Status) "NewEnumerator2")
          (if (> (.Z (Math|Vector|BreakVector (Transformation|GetWorldLocation _array_element))) (.z (+ (Variables|Default|GetElevator%20Start%20Location) (Math|Vector|MakeVector 0.0 0.0 _distance_to_travel))))
            (Rendering|SetVisibility _array_element false false)
            (else
              (Rendering|SetVisibility _array_element true false :!label _label)))
          (else
            (goto _label)))))
    (:Finished
      (if (Utilities|Enum|Equal(Enum) (Variables|Initialization|GetElevator%20Status) "NewEnumerator2")
        (bind _output_get (Variables|Initialization|SetElevator%20Status "NewEnumerator3"))
        (Default|CallOnElevatorStatusChanged _output_get)
        (else
          (bind _output_get_2 (Variables|Initialization|SetElevator%20Status "NewEnumerator0"))
          (Default|CallOnElevatorStatusChanged _output_get_2)))
      (Variables|Default|SetElevator%20Start%20Location (Transformation|GetWorldLocation (Variables|Default|GetSM_Elevator_1))))))

(event Custom|Create%20All%20Static%20Mesh%20Components%20Needed
  (bind _chain_length (Variables|Default|GetChain%20Length))
  (Variables|Default|SetElevator%20Start%20Location (Transformation|GetWorldLocation (Variables|Default|GetSM_Elevator_1)))
  (for _array_element (Actor|GetComponentsbyTag "/Script/Engine.StaticMeshComponent" "Chain")
    (Utilities|IsValid (Variables|/Script/Engine.StaticMeshComponent|GetStaticMesh _array_element)
      (:Is%20Valid
        (for _index (range 0 (- (Math|Float|Truncate (/ (Math|Vector|Distance(Vector) (Math|Vector|MakeVector 0.0 0.0 (.Z (Math|Vector|BreakVector (Variables|Initialization|GetChain%20End%20Location)))) (Math|Vector|MakeVector 0.0 0.0 (.Z (Math|Vector|BreakVector (- (Variables|/Script/Engine.SceneComponent|GetRelativeLocation _array_element) (Math|Vector|MakeVector 0.0 0.0 (/ (Variables|Default|GetChain%20Length) 2.0))))))) (Variables|Default|GetChain%20Length))) 2))
          (bind _returnvalue (AddComponent|AddStaticMeshComponent false))
          (Transformation|SetWorldLocation _returnvalue (Math|Vector|MakeVector (.x (Transformation|GetWorldLocation _array_element)) (.y (Transformation|GetWorldLocation _array_element)) (+ (.z (Transformation|GetWorldLocation _array_element)) (* _index _chain_length) _chain_length 0.0)) false true)
          (Transformation|AttachComponentToComponent _returnvalue (Variables|Default|GetSM_Elevator_1) "None" "KeepWorld" "KeepWorld" "KeepWorld" true)
          (Utilities|Array|Add (Variables|Default|GetAll%20Static%20Meshes) _returnvalue)
          (Transformation|SetWorldRotation _returnvalue (Transformation|GetWorldRotation _array_element) false false)
          (Components|StaticMesh|SetStaticMesh _returnvalue (Variables|/Script/Engine.StaticMeshComponent|GetStaticMesh _array_element)))
        (for _array_element_2 (Variables|Default|GetAll%20Static%20Meshes)
          (if (> (.Z (Math|Vector|BreakVector (Transformation|GetWorldLocation _array_element_2))) (.z (+ (Variables|Default|GetElevator%20Start%20Location) (Math|Vector|MakeVector 0.0 0.0 (Variables|Initialization|GetDistance%20To%20Travel)))))
            (Rendering|SetVisibility _array_element_2 false false)
            (else
              (Rendering|SetVisibility _array_element_2 true false))))))))

(event EventBeginPlay
  (EventDispatchers|BindEventtoOnElevatorStatusChanged (delegate Custom|On%20Elevator%20Status%20Changed_Event))
  (CallFunction|CreateAllStaticMeshComponentsNeeded))

(fn ConstructionScript
  (bind _spotlight (Variables|Default|GetSpotLight))
  (if (Variables|Default|GetUse%20Spotlight?)
    (Rendering|SetVisibility _spotlight true false)
    (else
      (Rendering|SetVisibility _spotlight false false))))