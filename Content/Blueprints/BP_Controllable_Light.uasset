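; BP_Controllable_Light is an actor, named as a light, that the player rotates with the mouse.
; On BeginPlay it passes itself to LE_PlayerController's SetInputPlayer, and right mouse press and release toggle IsRotating, with debug prints.
; While that flag and HorrorEngineCharacter's TryToRotateLight are both true, horizontal mouse movement sets the yaw from scaled, inverted input plus the actor's current roll, rather than its current yaw.
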(event EventBeginPlay
  (Default|SetInputPlayer (.AsLE%20Player%20Controller (Utilities|Casting|CastToLE_PlayerController (Game|GetPlayerController 0))) self))

(event Input|MouseEvents|MouseX
  (params (AxisValue :type Float%20%28single-precision%29))
  (if (Variables|/Game/HorrorEngine/Blueprints/Core/HorrorEngineCharacter.HorrorEngineCharacter_C|GetTryToRotateLight (.AsHorror%20Engine%20Character (Utilities|Casting|CastToHorrorEngineCharacter (Game|GetPlayerCharacter 0))))
    (if (Variables|Default|GetIsRotating)
      (Development|PrintString "IsRotating!")
      (Transformation|SetActorRotation (Math|Rotator|MakeRotator 0.0 0.0 (+ (* AxisValue -3.0) (.roll (Transformation|GetActorRotation))))))))

(event Input|MouseEvents|RightMouseButton
  (params (Key :type Key%20Structure :default "None"))
  (:Pressed
    (Variables|Default|SetIsRotating true)
    (Development|PrintString "Set isRotating"))
  (:Released
    (Variables|Default|SetIsRotating false)))

(fn ConstructionScript
  (|CallParentFunction))