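; BP_Door_1 is an interactive double door that the player opens and closes with the E key.
; A timeline drives opposite yaw rotations on the left and right door meshes at fixed relative locations, playing to open and reversing to close.
; Tick derives DoorClosed from the timeline alpha.
; The trigger enables player input on both begin and end overlap, so input is never disabled on leaving.
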(event OnComponentBeginOverlap(Trigger)
  (params (OverlappedComponent :type Primitive%20Component%20Object%20Reference) (OtherActor :type Actor%20Object%20Reference) (OtherComp :type Primitive%20Component%20Object%20Reference) (OtherBodyIndex :type Integer) (bFromSweep :type Boolean) (SweepResult :type Hit%20Result%20Structure%20%28by%20ref%29))
  (Input|EnableInput (Game|GetPlayerController 0)))

(event OnComponentEndOverlap(Trigger)
  (params (OverlappedComponent :type Primitive%20Component%20Object%20Reference) (OtherActor :type Actor%20Object%20Reference) (OtherComp :type Primitive%20Component%20Object%20Reference) (OtherBodyIndex :type Integer))
  (Input|EnableInput (Game|GetPlayerController 0)))

(event EventBeginPlay)

(event Collision|EventActorBeginOverlap
  (params (OtherActor :type Actor%20Object%20Reference)))

(event EventTick
  (params (DeltaSeconds :type Float%20%28single-precision%29))
  (Variables|Default|SetDoor%20Closed? (< (stale Input|KeyboardEvents|E _alpha) 1.0)))

(event Input|KeyboardEvents|E
  (params (Key :type Key%20Structure :default "None"))
  (:Pressed
    (if (Variables|Default|GetDoor%20Closed?)
      (bind _alpha (Timeline|Timeline Play)
        (:Update
          (Transformation|SetRelativeLocationAndRotation (Variables|Default|GetSM_Door_1_L) "0.000000,-114.000000,170.000000" (Math|Rotator|MakeRotator 0.0 0.0 _alpha) false false)
          (Transformation|SetRelativeLocationAndRotation (Variables|Default|GetSM_Door_1_R) "0.000000,99.000000,170.000000" (* (Math|Rotator|MakeRotator 0.0 0.0 _alpha) -1.0) false false)))
      (else
        (Timeline|Timeline Reverse)))))

(fn ConstructionScript)